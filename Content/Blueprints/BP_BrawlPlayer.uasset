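; BP_BrawlPlayer is a brawler player Blueprint that can punch other players.
; Punch input calls a PunchStart dispatcher, which enables query-only collision on a hand Sphere; a bound PunchEnd event disables it.
; Sphere overlaps print the other actor's name and pass movement velocity to its GetPunched.
; GetPunched is currently empty, with disconnected nodes for falling and applying force to the mesh.
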(event OnComponentBeginOverlap(Sphere)
  (params (OverlappedComponent :type Primitive%20Component%20Object%20Reference) (OtherActor :type Actor%20Object%20Reference) (OtherComp :type Primitive%20Component%20Object%20Reference) (OtherBodyIndex :type Integer) (bFromSweep :type Boolean) (SweepResult :type Hit%20Result%20Structure%20%28by%20ref%29))
  ;[1 1 1] Check punch
  (if (!= OtherActor self)
    (Development|PrintString (Utilities|GetDisplayName OtherActor))
    (bind _returnvalue (Class|BrawlerMovementComponent|GetVelocity (Variables|Default|GetMovementComponent)))
    (CallFunction|GetPunched (.AsBP%20Brawl%20Player (Utilities|Casting|CastToBP_BrawlPlayer OtherActor)) _returnvalue)))

(event Custom|OnPunchStart
  ;[1 1 1] On Punch Start
  (Collision|SetCollisionEnabled (Variables|Punch|GetSphere) "QueryOnly"))

(event Custom|PunchEnd_Event_0
  ;[1 1 1] On Punch End
  (Collision|SetCollisionEnabled (Variables|Punch|GetSphere) "NoCollision"))

(event EventBeginPlay
  ;[1 1 1] Begin Play. Binding events and turning off collision on the punching hand
  (EventDispatchers|AssignPunchEnd (delegate Custom|PunchEnd_Event_0))
  (EventDispatchers|BindEventtoPunchStart (delegate Custom|OnPunchStart))
  (Collision|SetCollisionEnabled (Variables|Punch|GetSphere) "NoCollision"))

(event Input|ActionEvents|InputActionPunch
  (params (Key :type Key%20Structure))
  ;[1 1 1] Input
  (:Pressed
    (Default|CallPunchStart)))

(fn ConstructionScript)

(fn GetPunched
  (params (Force :type Vector)))