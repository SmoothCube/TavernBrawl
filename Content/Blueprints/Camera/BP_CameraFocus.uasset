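; BP_CameraFocus is a shared camera actor that frames the first two BP_BrawlPlayer actors.
; On BeginPlay it becomes the view target of every BP_BrawlPC and caches the player actors.
; Each tick it moves to the midpoint between the two players and sets the spring arm length to their separation, with a minimum length so the view does not get too close.
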(event EventBeginPlay
  (bind _outactors (Actor|GetAllActorsOfClass "/Game/Blueprints/BP_BrawlPC.BP_BrawlPC_C"))
  (for _array_element _outactors
    (Game|Player|SetViewTargetwithBlend _array_element self 0.0 "VTBlend_Linear" 0.0 false)
    (bind _outactors_2 (Actor|GetAllActorsOfClass "/Game/Blueprints/BP_BrawlPlayer.BP_BrawlPlayer_C"))
    (Variables|Default|SetPlayers _outactors_2)))

(event EventTick
  (params (DeltaSeconds :type Float%20%28single-precision%29))
  (bind _players (Variables|Default|GetPlayers))
  (bind _springarm (Variables|Default|GetSpringArm))
  (bind _output (Utilities|Array|Get(acopy) _players 1))
  (bind _returnvalue (Transformation|GetActorLocation _output))
  (bind _output_get (Variables|CameraLocation|SetDistance (- (Transformation|GetActorLocation (Utilities|Array|Get(acopy) _players)) _returnvalue)))
  (Transformation|SetActorLocation (+ _returnvalue (/ _output_get 2)) false false)
  (if (< (Math|Vector|VectorLength _output_get) (Variables|Default|GetSmallestSpringArmLength))
    (Variables|/Script/Engine.SpringArmComponent|SetTargetArmLength _springarm (Variables|Default|GetSmallestSpringArmLength))
    (else
      (Variables|/Script/Engine.SpringArmComponent|SetTargetArmLength _springarm (Math|Vector|VectorLength _output_get)))))

(fn ConstructionScript)